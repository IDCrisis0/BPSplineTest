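; PipeGenerator is a Blueprint that lays out a pipe along a spline in the construction script.
; It adds a spline mesh component per spline index, joining each point to the next by location and tangent, with no static mesh assigned.
; It then grows or trims PipeDataArray to match the point count.
; BuildPipeElement is an uncalled, unfinished helper that only caches segment endpoints and tangents.
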(event EventBeginPlay)

(event Collision|EventActorBeginOverlap
  (params (OtherActor :type Actor%20Object%20Reference)))

(event EventTick
  (params (DeltaSeconds :type Float%20%28single-precision%29)))

(fn ConstructionScript
  (bind _pipespline (Variables|Default|GetPipeSpline))
  (bind _pipespline_2 (Variables|Default|GetPipeSpline))
  (bind _returnvalue (Spline|GetNumberOfSplinePoints _pipespline_2))
  (Utilities|FlowControl|Sequence
    (:then_0
      (Variables|Default|SetNumSplinePoints _returnvalue)
      (for _index (range 0 _returnvalue)
        (bind _returnvalue_2 (AddComponent|AddSplineMeshComponent false))
        (Components|StaticMesh|SetStaticMesh _returnvalue_2 0)
        (SplineMesh|SetStartandEnd _returnvalue_2 (.Location (Spline|GetLocationandTangentatSplinePoint _pipespline _index "Local")) (.Tangent (Spline|GetLocationandTangentatSplinePoint _pipespline _index "Local")) (.Location (Spline|GetLocationandTangentatSplinePoint _pipespline (+ _index 1) "Local")) (.Tangent (Spline|GetLocationandTangentatSplinePoint _pipespline (+ _index 1) "Local")) true :!class /Script/Engine.SplineMeshComponent)))
    (:then_1
      (|BuildsRoadDataArray))))

(fn BuildPipeElement
  (params (LoopIndex :type Integer) (PipeElementMesh :type Static%20Mesh%20Object%20Reference))
  (LocalVariables|SetL_CurrentLoopIndex LoopIndex)
  (LocalVariables|SetL_NextLoopIndex (Math|Integer|%(Integer) (+ LoopIndex 1) (LocalVariables|GetL_CurrentLoopIndex)))
  (LocalVariables|SetL_TrackElementMesh PipeElementMesh)
  (Utilities|FlowControl|Sequence
    (:then_0
      (LocalVariables|SetL_StartLocation (.Location (Spline|GetLocationandTangentatSplinePoint (Variables|Default|GetPipeSpline) (LocalVariables|GetL_CurrentLoopIndex) "Local")))
      (LocalVariables|SetL_StartTangent (.Tangent (Spline|GetLocationandTangentatSplinePoint (Variables|Default|GetPipeSpline) (LocalVariables|GetL_CurrentLoopIndex) "Local")))
      (LocalVariables|SetL_EndLocation (.Location (Spline|GetLocationandTangentatSplinePoint (Variables|Default|GetPipeSpline) (LocalVariables|GetL_NextLoopIndex) "Local")))
      (LocalVariables|SetL_EndTangent (.Tangent (Spline|GetLocationandTangentatSplinePoint (Variables|Default|GetPipeSpline) (LocalVariables|GetL_NextLoopIndex) "Local"))))))